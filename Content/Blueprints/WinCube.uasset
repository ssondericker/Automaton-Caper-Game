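; WinCube is an exit trigger actor that handles the win condition when a Crew overlaps it.
; On BeginPlay it creates the MyHUD widget and adds it to the viewport.
; On overlap it sets the HUD's exited flag and copies the crew's research state into it.
; If the crew has research, it waits briefly, pauses the game and plays win and success voice sounds.
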(event `self.ReceiveBeginPlay`
  (bind _returnvalue (`|CreateWidget` "/Game/View/MyHUD.MyHUD_C"))
  (`UserWidget.AddToViewport` _returnvalue 0)
  (set `self.MyHUD` _returnvalue))

(event `self.ReceiveActorBeginOverlap`
  (params (OtherActor :type "Actor Object Reference"))
  (bind _myhud (`self.MyHUD`))
  (bind _ascrew (cast `/Game/Character/Crew/Crew` OtherActor))
  (set `/Game/View/MyHUD.HasExited` true _myhud)
  (bind _output_get (set `/Game/View/MyHUD.HasReasearch` (`/Game/Character/Crew/Crew.HasResearch` _ascrew) _myhud))
  (if _output_get
    (`KismetSystemLibrary.Delay` 0.5)
    (`GameplayStatics.SetGamePaused` true)
    (`GameplayStatics.PlaySound2D` "/Game/Audio/WinSound.WinSound" 1.0 1.0 0.0 null null)
    (`GameplayStatics.PlaySound2D` "/Game/Audio/SuccessVoice.SuccessVoice" 1.0 1.0 0.0 null null)))

(fn `UserConstructionScript`)