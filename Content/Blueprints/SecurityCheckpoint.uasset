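; Security checkpoint actor that blocks the way with doors until a widget-driven challenge, configured with per-instance hints and solutions, is passed.
; A Crew overlap disables Robot movement and starts the widget's protocol, which Tick runs and polls for the result.
; Passing plays sounds, hides sparkle flipbooks, restores Robots to flying and slides one or two doors open by delayed timeline, removing collision.
; Failing flags the first Robot found as failed.
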(event `self.ReceiveBeginPlay`
  (bind _checkpointwidget (`self.CheckpointWidget`))
  (bind _returnvalue (`|CreateWidget` "/Game/View/SecurityCheckpointWidget.SecurityCheckpointWidget_C"))
  (`UserWidget.AddToViewport` _returnvalue 10)
  (set `self.CheckpointWidget` _returnvalue)
  (set `self.door_start_location` (`self.K2_GetActorLocation` (`self.door`)))
  (set `self.doorstartlocation2` (`self.K2_GetActorLocation` (`self.door2`)))
  (set `/Game/View/SecurityCheckpointWidget.HintStrings` (`self.HintStringsBP`) _checkpointwidget)
  (set `/Game/View/SecurityCheckpointWidget.Solutions` (`self.Solutions_BP`) _checkpointwidget))

(event `self.ReceiveActorBeginOverlap`
  (params (OtherActor :type "Actor Object Reference"))
  (cast `/Game/Character/Crew/Crew` OtherActor)
  (set `/Game/View/SecurityCheckpointWidget.IsAtCheckpoint` true (`self.CheckpointWidget`))
  (set `self.started` true)
  (bind _outactors (`GameplayStatics.GetAllActorsOfClass` "/Game/Character/Robot/Robot.Robot_C"))
  (for _array_element _outactors
    (`CharacterMovementComponent.DisableMovement` (`Character.CharacterMovement` _array_element))))

(event `self.ReceiveTick`
  (params (DeltaSeconds :type "Float (single-precision)"))
  (bind _checkpointwidget (`self.CheckpointWidget`))
  ;[1 1 1] event tick
  (if (`self.started`)
    (`/Game/View/SecurityCheckpointWidget.SCProtocol` (`self.CheckpointWidget`))
    (if (`/Game/View/SecurityCheckpointWidget.FinishedCheckpoint` _checkpointwidget)
      (if (`/Game/View/SecurityCheckpointWidget.PassedCheckpoint` _checkpointwidget)
        (if (not (`self.cleared`))
          (set `self.cleared` true)
          (`GameplayStatics.PlaySound2D` "/Game/Audio/CheckpointCleared.CheckpointCleared" 1.0 1.0 0.0 null null)
          (`self.move door`)
          (`self.Remove sparkles`)
          (`KismetSystemLibrary.Delay` 0.8)
          (`GameplayStatics.PlaySound2D` "/Game/Audio/DoorOpen.DoorOpen" 1.0 1.0 0.0 null null)
          (bind _outactors (`GameplayStatics.GetAllActorsOfClass` "/Game/Character/Robot/Robot.Robot_C"))
          (for _array_element _outactors
            (`CharacterMovementComponent.SetMovementMode` (`Character.CharacterMovement` _array_element) "MOVE_Flying" 0)))
        (else
          (bind _outactors_2 (`GameplayStatics.GetAllActorsOfClass` "/Game/Character/Robot/Robot.Robot_C"))
          (set `self.robot` (`|GetArrayItem` _outactors_2))
          (set `/Game/Character/Robot/Robot.FailedCheckpoint` true (`self.robot`)))))))

(event `Remove sparkles`
  ;[1 1 1] remove sparkles
  (for _array_element (`self.sparkles`)
    (`SceneComponent.SetVisibility` (`/Game/Blueprints/BP_sparkle_FB.PaperFlipbook` _array_element) false false)))

(event `move door`
  ;[1 1 1] move door
  (`KismetSystemLibrary.Delay` 2.2)
  (bind (_direction _move_door _move_door_2) (`Timeline|MoveDoor`)
    (:`Update`
      (if (`self.door_vert`)
        (`self.K2_SetActorRelativeLocation` (`self.door2`) (+ _move_door_2 (`self.doorstartlocation2`)) false false :!label _label)
        (`PrimitiveComponent.SetCollisionEnabled` (`/Game/Blueprints/wall_vertical.PaperSprite` (`self.door2`)) "NoCollision")
        (else
          (`self.K2_SetActorRelativeLocation` (`self.door`) (+ _move_door (`self.door_start_location`)) false false)
          (if (`self.2doors`)
            (goto _label)
            (else
              _))))
      (`PrimitiveComponent.SetCollisionEnabled` (`self.Box`) "NoCollision")
      (`PrimitiveComponent.SetCollisionEnabled` (`/Game/Blueprints/wall_vertical.PaperSprite` (`self.door`)) "NoCollision"))))

(fn `UserConstructionScript`)